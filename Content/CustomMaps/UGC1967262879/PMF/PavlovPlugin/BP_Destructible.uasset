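; Replicated destructible prop for a Pavlov custom map that shatters when damaged and restores itself each round.
; The first damage event after a reset passes a DoOnce and sets Destroyed if it meets a minimum amount.
; The RepNotify fractures the mesh with radius damage and disables Box collision, or restores both when cleared at round start.
; BeginPlay reapplies the broken state if Destroyed is already set.
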(event EventBeginPlay
  (if (Variables|Default|GetDestroyed?)
    (Class|DestructibleComponent|ApplyRadiusDamage (Variables|Default|GetDestructible) 1e+02 (+ (Transformation|GetWorldLocation (Variables|Default|GetDestructible)) 1.0) 5e+01 1e+02 true)
    (Collision|SetCollisionEnabled (Variables|Default|GetBox) "NoCollision")))

(event EventRoundStarting
  (Variables|Default|SetDestroyed? false)
  (Utilities|FlowControl|DoOnce false) ; enters at Reset
)

(event Game|Damage|EventAnyDamage
  (params (Damage :type Float%20%28single-precision%29) (DamageType :type Damage%20Type%20Object%20Reference) (InstigatedBy :type Controller%20Object%20Reference) (DamageCauser :type Actor%20Object%20Reference))
  (Utilities|FlowControl|DoOnce false
    (:Completed
      (Variables|Default|SetDestroyed? (>= Damage 1.0)))))

(fn ConstructionScript)

(fn OnRepDestroyed?
  (if (Variables|Default|GetDestroyed?)
    (Class|DestructibleComponent|ApplyRadiusDamage (Variables|Default|GetDestructible) 1e+02 (+ (Transformation|GetWorldLocation (Variables|Default|GetDestructible)) 1.0) 5e+01 1e+02 true)
    (Collision|SetCollisionEnabled (Variables|Default|GetBox) "NoCollision")
    (else
      (Class|DestructibleComponent|SetDestructibleMesh (Variables|Default|GetDestructible) (Variables|Default|GetDestructibleMesh))
      (Collision|SetCollisionEnabled (Variables|Default|GetBox) "QueryAndPhysics"))))