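; PMF_CharacterProxyInfo is a per-player proxy actor in the PMF framework that manages a character's custom VR hands, info actor and death state.
; On BeginPlay, the server spawns left and right hands linked to the motion controllers' owners, while clients optionally spawn player info for non-local players.
; PlayerDied destroys the hands and sets IsDead, whose RepNotify removes the player info.
; The proxy destroys itself when its player leaves.
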(event EventBeginPlay
  (|CallParentFunction)
  (if (Networking|IsServer)
    (CallFunction|ServerInitialization)
    (else
      (CallFunction|ClientInitialization))))

(fn ConstructionScript
  (|CallParentFunction))

(fn SpawnPlayerInfo
  (if (Variables|/Game/CustomMaps/UGC1967262879/PMF/Blueprints/LevelActors/CORE/PMF_GameLogic.PMF_GameLogic_C|GetbUsePMFPlayerInfo (CallFunction|GetPMFGameLogic))
    (if (not (Default|IsLocalPRI (Variables|DataReplicated|GetOwningPRI)))
      (Utilities|IsValid (Variables|Data|GetSpawnedPlayerInfo)
        (:Is%20Not%20Valid
          (bind _returnvalue (Game|SpawnActorfromClass (Variables|ConfigClass|GetPlayerInfoClass) (Math|Transform|MakeTransform "0, 0, 0") "AlwaysSpawn" 0 (Variables|DataReplicated|GetOwningPRI) 0))
          (Variables|Data|SetSpawnedPlayerInfo _returnvalue))))))

(fn OnRepBIsDead
  (Creation|DestroyPlayerInfo))

(fn DestroyPlayerInfo
  (Utilities|IsValid (Variables|Data|GetSpawnedPlayerInfo)
    (:Is%20Valid
      (Actor|DestroyActor (Variables|Data|GetSpawnedPlayerInfo)))))

(fn PlayerDied
  (Variables|DataReplicated|SetbIsDead true)
  (Creation|DestroyCustomHands))

(fn PlayerLeftServer
  (Actor|DestroyActor))

(fn SpawnCustomHands
  (bind _returnvalue (Math|Transform|MakeTransform "0, 0, 0"))
  (bind _customhandclass (Variables|ConfigClass|GetCustomHandClass))
  (bind _owningpri (Variables|DataReplicated|GetOwningPRI))
  (bind _owningpri_2 (Variables|DataReplicated|GetOwningPRI))
  (bind (_leftmotioncontroller _rightmotioncontroller) (Default|GetControllers _owningpri))
  (bind _pc (Default|GetPlayerController _owningpri_2))
  (if (Networking|IsServer)
    (Creation|DestroyCustomHands)
    (bind _returnvalue_2 (Game|SpawnActorfromClass _customhandclass _returnvalue "AlwaysSpawn" _pc true (Variables|DataReplicated|GetOwningPRI) (Components|GetOwner _rightmotioncontroller) self 0))
    (Variables|DataReplicated|SetPMFCustomHandR _returnvalue_2)
    (bind _returnvalue_3 (Game|SpawnActorfromClass _customhandclass _returnvalue "AlwaysSpawn" _pc false (Variables|DataReplicated|GetOwningPRI) (Components|GetOwner _leftmotioncontroller) self 0))
    (Variables|DataReplicated|SetPMFCustomHandL _returnvalue_3)
    (else
      (CallFunction|AddPMFLog "PMF Custom Hands are to be spawned on the server only!"))))

(fn DestroyCustomHands
  (bind _pmfcustomhandr (Variables|DataReplicated|GetPMFCustomHandR))
  (bind _pmfcustomhandl (Variables|DataReplicated|GetPMFCustomHandL))
  (Utilities|FlowControl|Sequence
    (:then_0
      (Utilities|IsValid _pmfcustomhandr
        (:Is%20Valid
          (Actor|DestroyActor _pmfcustomhandr))))
    (:then_1
      (Utilities|IsValid _pmfcustomhandl
        (:Is%20Valid
          (Actor|DestroyActor _pmfcustomhandl))))))

(fn GetOwningPRI
  (Utilities|IsValid (Variables|DataReplicated|GetOwningPRI)
    (:Is%20Valid
      (return true (Variables|DataReplicated|GetOwningPRI)))
    (:Is%20Not%20Valid
      (return false 0))))

(fn GetOwningCharacter
  (Utilities|IsValid (Variables|DataReplicated|GetOwningCharacter)
    (:Is%20Valid
      (return true (Variables|DataReplicated|GetOwningCharacter)))
    (:Is%20Not%20Valid
      (return false 0))))

(fn GetIsDead
  (return (Variables|DataReplicated|GetbIsDead)))

(fn GetCustomHands
  (if (and (Utilities|IsValid (Variables|DataReplicated|GetPMFCustomHandR)) (Utilities|IsValid (Variables|DataReplicated|GetPMFCustomHandL)))
    (return true (Variables|DataReplicated|GetPMFCustomHandR) (Variables|DataReplicated|GetPMFCustomHandL))
    (else
      (return false 0 0))))

(fn ServerInitialization
  (Creation|SpawnCustomHands))

(fn ClientInitialization
  (Creation|SpawnPlayerInfo))