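; Replication info object for one squad in the PMF game mode, tracking member PRIs, leader, lock state, score and wins.
; Joining assigns the squad index and promotes the first member; leaving re-promotes if needed or unlocks an empty squad.
; Queries report living members and slots left against the game logic's MaxSquadSize.
; Lock changes and promotion are server-gated, but the leader assignment in PromoteSquadLeader is disconnected and never runs.
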(fn ConstructionScript)

(fn PlayerJoinSquad
  (params (PRI :type PMF%20Player%20Replication%20Info%20Object%20Reference))
  (Utilities|Array|AddUnique (Variables|DataReplicated|GetSquadPRIs) PRI)
  (Default|SetSquadIndex PRI (Variables|DataReplicated|GetSquadIndex))
  (if (== (Utilities|Array|Length (Variables|DataReplicated|GetSquadPRIs)) 1)
    (SquadLeader|PromoteSquadLeader PRI)))

(fn PlayerLeaveSquad
  (params (PRI :type PMF%20Player%20Replication%20Info%20Object%20Reference))
  (Utilities|FlowControl|Sequence
    (:then_0
      (Utilities|Array|RemoveItem (Variables|DataReplicated|GetSquadPRIs) PRI))
    (:then_1
      (if (Info|HasAnyPlayers)
        (if (or (not (Utilities|IsValid (Variables|DataReplicated|GetSquadLeaderPRI))) (== (Variables|DataReplicated|GetSquadLeaderPRI) PRI))
          (SquadLeader|PromoteSquadLeader (Utilities|Array|Get(acopy) (Variables|DataReplicated|GetSquadPRIs))))
        (elif (Getters|IsSquadLocked)
          (Locking|UnlockSquad))))))

(fn GetPlayerCount
  (return (Utilities|Array|Length (Variables|DataReplicated|GetSquadPRIs))))

(fn HasAnyPlayers
  (return (> (Getters|GetPlayerCount) 0)))

(fn SetSquadScore
  (params (NewScore :type Integer))
  (Variables|DataReplicated|SetSquadScore NewScore))

(fn SetSquadWins
  (params (NewWins :type Integer))
  (Variables|DataReplicated|SetSquadWins NewWins))

(fn AddSquadScore
  (params (AdditionalScore :type Integer))
  (Variables|DataReplicated|SetSquadScore (+ AdditionalScore (Variables|DataReplicated|GetSquadScore))))

(fn AddSquadWins
  (params (AdditionalWins :type Integer))
  (Variables|DataReplicated|SetSquadWins (+ AdditionalWins (Variables|DataReplicated|GetSquadWins))))

(fn IncrementSquadScore
  (Math|Integer|IncrementInt (Variables|DataReplicated|GetSquadScore)))

(fn IncrementSquadWins
  (Math|Integer|IncrementInt (Variables|DataReplicated|GetSquadWins)))

(fn GetSquadScore
  (return (Variables|DataReplicated|GetSquadScore)))

(fn HasAlivePlayers
  (for _array_element (Variables|DataReplicated|GetSquadPRIs)
    (if (not (Default|IsDead _array_element))
      (return true)))
  (return false))

(fn GetSquadWins
  (return (Variables|DataReplicated|GetSquadWins)))

(fn GetSquadName
  (return (Variables|DataReplicated|GetSquadName)))

(fn IsSquadLocked
  (return (Variables|DataReplicated|GetbSquadIsLocked)))

(fn LockSquad
  (if (Networking|IsServer)
    (Variables|DataReplicated|SetbSquadIsLocked true)))

(fn UnlockSquad
  (if (Networking|IsServer)
    (Variables|DataReplicated|SetbSquadIsLocked false)))

(fn PromoteSquadLeader
  (params (PRI :type PMF%20Player%20Replication%20Info%20Object%20Reference))
  (if (Networking|IsServer)
    (Utilities|IsValid PRI
      (:Is%20Valid
        (if (!= PRI (Variables|DataReplicated|GetSquadLeaderPRI))
          _)))))

(fn GetSquadLeaderPRI
  (return (Variables|DataReplicated|GetSquadLeaderPRI)))

(fn IsSquadLeader
  (params (PRI :type PMF%20Player%20Replication%20Info%20Object%20Reference))
  (return (and (Utilities|IsValid (Variables|DataReplicated|GetSquadLeaderPRI)) (== (Variables|DataReplicated|GetSquadLeaderPRI) PRI))))

(fn GetSlotsLeft
  (return (- (Variables|/Game/CustomMaps/UGC1967262879/PMF/Blueprints/LevelActors/CORE/PMF_GameLogic.PMF_GameLogic_C|GetMaxSquadSize (CallFunction|GetPMFGameLogic)) (Getters|GetPlayerCount))))

(fn HasSlotsLeft
  (return (> (Info|GetSlotsLeft) 0)))