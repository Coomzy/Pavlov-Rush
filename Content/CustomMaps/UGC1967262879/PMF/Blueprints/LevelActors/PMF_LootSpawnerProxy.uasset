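; PMF_LootSpawnerProxy is a loot spawner proxy level actor that builds its spawn list from an enum list of item types.
; When SpawnListEnum has entries, the construction script rebuilds SpawnList as unique strings, first resolving random item types to a type via RandomItemToType.
; It then runs the parent construction script; the event graph holds no active logic.
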(event EventBeginPlay)

(event Collision|EventActorBeginOverlap
  (params (OtherActor :type Actor%20Object%20Reference)))

(event EventTick
  (params (DeltaSeconds :type Float%20%28single-precision%29)))

(fn ConstructionScript
  (if (> (Utilities|Array|Length (Variables|LootSpawnSettings|GetSpawnListEnum)) 0)
    (Utilities|Array|Clear (Variables|Default|GetSpawnList))
    (for _array_element (Variables|LootSpawnSettings|GetSpawnListEnum)
      (bind _bisrandom (CallFunction|IsItemTypeRandom _array_element))
      (if _bisrandom
        (bind _itemname (CallFunction|RandomItemtoType _array_element))
        (Utilities|Array|AddUnique (Variables|Default|GetSpawnList) (Utilities|String|EnumtoString _itemname))
        (else
          (Utilities|Array|AddUnique (Variables|Default|GetSpawnList) (Utilities|String|EnumtoString _array_element))))))
  (|CallParentFunction))