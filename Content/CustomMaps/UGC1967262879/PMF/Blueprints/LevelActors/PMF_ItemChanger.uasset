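; Level actor that finds configured items, or other non-item classes, in the world and spawns a mesh swapper actor owned by each instance.
; An interval Tick, intended for clients only, alternates between scanning for new matches and pruning invalid cache entries.
; ItemCache prevents duplicate swappers.
; Delayed and manual refresh entry points run extra scans, skipped on dedicated servers.
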(event Custom|DelayedRefresh
  (params (Delay :type Float%20%28single-precision%29))
  (if (not (Networking|IsDedicatedServer))
    (Utilities|FlowControl|Delay Delay)
    (CallFunction|DoItemChecks)))

(event EventTick
  (params (DeltaSeconds :type Float%20%28single-precision%29))
  (bind _output_get (Variables|Data|SetbHasDoneHalfway (not (Variables|Data|GetbHasDoneHalfway))))
  (if _output_get
    (CallFunction|DoItemChecks) ; Consider Splitting This Across Frames To Avoid Hitches
    (else
      (CallFunction|DoCleanUpChecks))))

(fn ConstructionScript)

(fn DoItemChecks
  (for _array_element (Variables|Config|GetItemsToSwap)
    (bind (_itemclass _bfound) (CallFunction|GetItemClassbyID (.ItemID (Utilities|Struct|BreakPMF_ItemMeshSwapperData _array_element))))
    (if (or _bfound (Utilities|Enum|Equal(Enum) (.ItemID (Utilities|Struct|BreakPMF_ItemMeshSwapperData _array_element)) "NewEnumerator43"))
      (if (!= (select (Utilities|Enum|Equal(Enum) (.ItemID (Utilities|Struct|BreakPMF_ItemMeshSwapperData _array_element)) "NewEnumerator43") (.NonItemClass (Utilities|Struct|BreakPMF_ItemMeshSwapperData _array_element)) _itemclass) 0)
        (bind _outactors (Actor|GetAllActorsOfClass (select (Utilities|Enum|Equal(Enum) (.ItemID (Utilities|Struct|BreakPMF_ItemMeshSwapperData _array_element)) "NewEnumerator43") (.NonItemClass (Utilities|Struct|BreakPMF_ItemMeshSwapperData _array_element)) _itemclass)))
        (for _array_element_2 _outactors
          (if (not (Utilities|Array|ContainsItem (Variables|Data|GetItemCache) _array_element_2))
            (Utilities|Array|Add (Variables|Data|GetItemCache) _array_element_2)
            (Game|SpawnActorfromClass (.ItemMeshSwapper (Utilities|Struct|BreakPMF_ItemMeshSwapperData _array_element)) (Math|Transform|MakeTransform "0, 0, 0") "AlwaysSpawn" _array_element_2 0)))))))

(fn DoCleanUpChecks
  (bind (_arrayindex _arrayelement) (Utilities|Array|ReverseforEachLoop (Variables|Data|GetItemCache))
    (:LoopBody
      (Utilities|IsValid _arrayelement
        (:Is%20Not%20Valid
          (Utilities|Array|RemoveIndex (Variables|Data|GetItemCache) _arrayindex))))))

(fn DoManualRefresh
  (if (not (Networking|IsDedicatedServer))
    (CallFunction|DoItemChecks)))