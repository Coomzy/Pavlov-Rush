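; Per-player info display actor for the PMF game mode that follows its owning player's head and exposes health percentage and same-team checks.
; Spawning shows it after a short replication delay, caching max health from PMF game logic; death or inactivity hides it.
; Tick snaps it to the head socket, yawed toward the local VR headset, or matching headset yaw for the local player's own.
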(event Custom|DelayedActivate
  (Utilities|FlowControl|Delay 0.5) ; Delay For Replication... this could be better
  (CallFunction|Activate))

(event EventBeginPlay
  (|CallParentFunction)
  (Development|SetHiddeninGame (Variables|Default|GetDefaultSceneRoot) true true)
  (if (.bIsValid (Default|GetPlayerCharacter (Variables|Data|GetOwningPRI)))
    (CallFunction|DelayedActivate)))

(event EventTick
  (params (DeltaSeconds :type Float%20%28single-precision%29))
  (|CallParentFunction DeltaSeconds)
  (if (not (Variables|Rendering|GetbHidden))
    (CallFunction|UpdateLocandRot)
    (if (Default|IsInactive (Variables|Data|GetOwningPRI))
      (CallFunction|Deactivate))))

(fn ConstructionScript)

(fn SetupPlayerInfo)

(fn PlayerSpawned
  (CallFunction|DelayedActivate))

(fn PlayerDied
  (CallFunction|Deactivate))

(fn IsonSameTeamasLocalPlayer
  (if (Utilities|Enum|Equal(Enum) (Variables|/Game/CustomMaps/UGC1967262879/PMF/Blueprints/LevelActors/CORE/PMF_GameLogic.PMF_GameLogic_C|GetPMFModeType (CallFunction|GetPMFGameLogic)) "NewEnumerator0")
    (return false)
    (else
      (return (== (Default|GetTeamIndex (CallFunction|GetLocalPRI)) (Default|GetTeamIndex (Variables|Data|GetOwningPRI)))))))

(fn GetHealthPct
  (bind _owningpri (Variables|Data|GetOwningPRI))
  (bind (_playerstatus _bsucceeded) (Default|GetPlayerStatus _owningpri))
  (bind (_health _bdead) (Utilities|Struct|BreakPavlovPlayerStatus _playerstatus))
  (if _bsucceeded
    (if _bdead
      (return 0.0)
      (else
        (return (Math|Float|Clamp(Float) (Math|Conversions|ToFloat(Integer) (/ _health (Variables|Data|GetMaxHealth)))))))
    (else
      (return 0.0))))

(fn Activate
  (bind _playersettings (Default|GetPlayerSettingsfor (CallFunction|GetPMFGameLogic) (Variables|Data|GetOwningPRI)))
  (Variables|Data|SetMaxHealth (.Health (Utilities|Struct|BreakPMF_PlayerSettingsData _playersettings)))
  (Development|SetHiddeninGame (Variables|Default|GetDefaultSceneRoot) false true))

(fn Deactivate
  (Development|SetHiddeninGame (Variables|Default|GetDefaultSceneRoot) true true))

(fn GetPlayerInfoWorldLoc
  (return (Transformation|GetWorldLocation (Variables|Default|GetOffsetRoot))))

(fn UpdateLocandRot
  (bind _localpri (CallFunction|GetLocalPRI))
  (bind _owningpri (Variables|Data|GetOwningPRI))
  (bind (_character _bisvalid) (Default|GetPlayerCharacter _owningpri))
  (bind _vrcamera (Default|GetVRHeadsetCamera _localpri))
  (if _bisvalid
    (Transformation|SetActorLocationAndRotation (Transformation|GetSocketLocation (Utilities|Array|Get(acopy) (Actor|GetComponentsByClass _character "/Script/Engine.SkeletalMeshComponent") (Variables|/Game/CustomMaps/UGC1967262879/PMF/Blueprints/Objects/PMF_PavlovIndexs.PMF_PavlovIndexs_C|GetInventoryCharacterBodyMeshOffset (CallFunction|GetPavlovIndexs))) "Head") (select (!= (Variables|Data|GetOwningPRI) (CallFunction|GetLocalPRI)) (Math|Conversions|RotationFromXVector (CallFunction|GetDirtoFlat (Transformation|GetWorldLocation _vrcamera) (CallFunction|GetPlayerInfoWorldLoc) true)) (Math|Rotator|MakeRotator 0.0 0.0 (.Yaw (Math|Rotator|BreakRotator (Transformation|GetWorldRotation _vrcamera))))))))