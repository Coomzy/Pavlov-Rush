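; Base pickup Blueprint that a player triggers by entering it, going inactive until a cooldown re-activates it.
; Enter events check replicated Active and Enabled flags, then UsePickup deactivates it and starts a server-side retriggerable delay.
; Only the server sets the flags; their OnRep functions and BeginPlay update the visual cube's visibility.
; An optional setting re-activates the pickup when a round starts.
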(event Custom|PickupCooldown
  (Utilities|ContinueifServer
    (:Server
      (Utilities|FlowControl|RetriggerableDelay (Variables|Config|GetResetDuration))
      (CallFunction|SetPickupActive true))))

(event EventBeginPlay
  (|CallParentFunction)
  (CallFunction|UpdatePickupVisibilityBasedonEnabledandActive))

(event EventRoundStarting
  (if (Variables|Config|GetbResetOnRoundStart)
    (CallFunction|SetPickupActive true)))

(event EventOnPlayerEnter
  (params (PRI :type PMF%20Player%20Replication%20Info%20Object%20Reference) (Pawn :type Pawn%20Object%20Reference))
  (|CallParentFunction PRI Pawn)
  (bind _bcanuse (CallFunction|CanUsePickup PRI))
  (if _bcanuse
    (CallFunction|UsePickup PRI)))

(fn ConstructionScript
  (|CallParentFunction))

(fn OnRepBIsPickupActive
  (CallFunction|UpdatePickupVisibilityBasedonEnabledandActive))

(fn OnRepBIsPickupEnabled
  (CallFunction|UpdatePickupVisibilityBasedonEnabledandActive))

(fn SetPickupEnabled
  (params (bEnable :type Boolean))
  (if (Networking|IsServer)
    (Variables|Config|SetbIsPickupEnabled bEnable)))

(fn SetPickupActive
  (params (bActive :type Boolean))
  (if (Networking|IsServer)
    (Variables|Config|SetbIsPickupActive bActive)))

(fn CanUsePickup
  (params (PRI :type PMF%20Player%20Replication%20Info%20Object%20Reference))
  (return (and (Variables|Config|GetbIsPickupActive) (Variables|Config|GetbIsPickupEnabled))))

(fn UsePickup
  (params (PRI :type PMF%20Player%20Replication%20Info%20Object%20Reference))
  (CallFunction|SetPickupActive false)
  (CallFunction|PickupCooldown))

(fn UpdatePickupVisibilityBasedonEnabledandActive
  (if (Variables|Config|GetbIsPickupEnabled)
    (Rendering|SetVisibility (Variables|Default|GetPlayerVisualCube) (Variables|Config|GetbIsPickupActive) false)
    (else
      (Rendering|SetVisibility (Variables|Default|GetPlayerVisualCube) false false))))