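; RSH_MCOM is a Rush-style bomb objective that attackers arm and defenders disarm before it detonates.
; Arming and disarming run locally, timed by sound length with cable visuals and range/death cancellation, then go through the player's PRI.
; The server owns armed and detonated state, runs the fuse and notifies the MCOM manager.
; Replicated start time syncs countdown audio, while a world widget turns, scales and rises with player distance.
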(event Custom|ArmedIntenseSoundTimer
  (Audio|Components|Audio|Stop (Variables|Default|GetAudioArmed))
  (Audio|Components|Audio|Play (Variables|Default|GetAudioArmedIntense) (- (Getters|GetArmedTime) (Getters|GetDetonationTime true)))
  (Utilities|FlowControl|RetriggerableDelay (Variables|/Script/Engine.SoundBase|GetDuration (Variables|/Script/Engine.AudioComponent|GetSound (Variables|Default|GetAudioArmedIntense))))
  (if (Variables|DataReplicated|GetbArmed)
    (Audio|Components|Audio|Stop (Variables|Default|GetAudioArmedIntense))))

(event Custom|DisarmingTimer
  (Utilities|FlowControl|RetriggerableDelay (Variables|/Script/Engine.SoundBase|GetDuration (Variables|/Script/Engine.AudioComponent|GetSound (Variables|Default|GetAudioDisarming))))
  (if (Getters|IsLocalDisarming)
    (LocalDisarming|FinishLocalDisarming)))

(event Custom|MulticastDisarm
  (Sounds|StopAllMCOMSounds)
  (Cable|StopCableVisual))

(event Custom|ArmingTimer
  (Utilities|FlowControl|RetriggerableDelay (Variables|/Script/Engine.SoundBase|GetDuration (Variables|/Script/Engine.AudioComponent|GetSound (Variables|Default|GetAudioArming))))
  (if (Getters|IsLocalArming)
    (LocalArming|FinishLocalArming)))

(event Custom|ArmedSoundTimer
  (Audio|Components|Audio|Play (Variables|Default|GetAudioArmed) (Getters|GetArmedTime))
  (Utilities|FlowControl|RetriggerableDelay (- (Variables|Config-RSH|GetDetonationTime) (Variables|/Script/Engine.SoundBase|GetDuration (Variables|/Script/Engine.AudioComponent|GetSound (Variables|Default|GetAudioArmedIntense)))))
  (if (Variables|DataReplicated|GetbArmed)
    (CallFunction|ArmedIntenseSoundTimer)))

(event Custom|MulticastRoundEnded
  (Sounds|StopAllMCOMSounds)
  (LocalArming|CancelLocalArming false)
  (LocalDisarming|CancelLocalDisarming false)
  (Cable|StopCableVisual))

(event Custom|ArmedTimer
  (Utilities|FlowControl|RetriggerableDelay (Variables|Config-RSH|GetDetonationTime))
  (if (Variables|DataReplicated|GetbArmed)
    (MainEvents|MCOMDetonate)))

(event Custom|MulticastDetonate
  (Audio|PlaySoundatLocation "/Game/CustomMaps/UGC1967262879/RSH/Audio/MCOM/MCOM-Explosion.MCOM-Explosion" (Transformation|GetActorLocation) "0, 0, 0" 1.0 1.0 0.0 0 0 0))

(event EventBeginPlay
  (|CallParentFunction)
  (Sounds|StopAllMCOMSounds)
  (Setup|SetupWidget)
  (Components|Activation|Deactivate (Variables|Default|GetCable_L)))

(event EventRoundStarting
  (MainEvents|RestoreMCOM))

(event EventTick
  (params (DeltaSeconds :type Float%20%28single-precision%29))
  (|CallParentFunction DeltaSeconds)
  (Widget|UpdateObjectiveWidget)
  (LocalArming|TrackLocalArming)
  (LocalDisarming|TrackLocalDisarming)
  (Visuals|UpdateArmedLight))

(event EventUseInteractableLocal
  (params (UserPRI :type PMF%20Player%20Replication%20Info%20Object%20Reference) (UserCPI :type PMF%20Character%20Proxy%20Info%20Object%20Reference) (UserCustomHand :type PMF%20Custom%20Hand%20Object%20Reference))
  (Cable|StartCableVisual UserCustomHand)
  (bind _asrsh_player_replication_info (Utilities|Casting|CastToRSH_PlayerReplicationInfo UserPRI))
  (if (Default|IsAttacker _asrsh_player_replication_info)
    (LocalArming|StartLocalArming _asrsh_player_replication_info)
    (else
      (LocalDisarming|StartLocalDisarming _asrsh_player_replication_info))))

(event EventRoundEnded
  (CallFunction|MulticastRoundEnded))

(fn ConstructionScript)

(fn StartLocalArming
  (params (RSHPRI :type RSH%20Player%20Replication%20Info%20Object%20Reference))
  (bind _bcanarm (LocalArming|CanDoLocalArming RSHPRI))
  (if _bcanarm
    (Variables|Data-LocalArming|SetLocalArmerRSHPRI RSHPRI)
    (Audio|Components|Audio|Play (Variables|Default|GetAudioArming) 0.0)
    (CallFunction|ArmingTimer)
    (CallFunction|AddPMFLog "Local Disarm Finish")))

(fn FinishLocalArming
  (Cable|StopCableVisual)
  (Utilities|IsValid (Variables|Data-LocalArming|GetLocalArmerRSHPRI)
    (:Is%20Valid
      (Default|ArmMCOM (Variables|Data-LocalArming|GetLocalArmerRSHPRI) (Getters|GetMCOMIndex))
      (Variables|Data-LocalArming|SetLocalArmerRSHPRI 0))))

(fn CancelLocalArming
  (params (bWasCanceledByPlayer :type Boolean))
  (Utilities|FlowControl|Sequence
    (:then_0
      (Audio|Components|Audio|Stop (Variables|Default|GetAudioArming))
      (Variables|Data-LocalArming|SetLocalArmerRSHPRI 0)
      (Cable|StopCableVisual))
    (:then_1
      (if bWasCanceledByPlayer
        (Audio|PlaySoundatLocation "/Game/CustomMaps/UGC1967262879/PMF/Audio/WINDOWS_XP_ERROR_SOUND.WINDOWS_XP_ERROR_SOUND" (Transformation|GetActorLocation) "0, 0, 0" 1.0 1.0 0.0 0 0 0)))))

(fn CanDoLocalArming
  (params (RSHPRI :type RSH%20Player%20Replication%20Info%20Object%20Reference))
  (if (not (Default|IsDead RSHPRI))
    (return true)
    (else
      (return false))))

(fn GetMCOMIndex
  (return (Variables|Config-RSH|GetMCOMIndex)))

(fn MCOMArmed
  (params (_ArmerRSHPRI :type RSH%20Player%20Replication%20Info%20Object%20Reference))
  (if (Networking|IsServer)
    (Variables|Data-ServerArming|SetArmerRSHPRI _ArmerRSHPRI)
    (Variables|DataReplicated|SetbArmed true)
    (Variables|DataReplicated|SetArmStartTime (GameState|GetServerWorldTimeSeconds (Game|GetGameState)))
    (CallFunction|ArmedTimer)))

(fn MCOMDetonate
  (bind (_mcommanager _bvalid) (CallFunction|GetMCOMManager))
  (if (Networking|IsServer)
    (Variables|DataReplicated|SetbDetonated true)
    (CallFunction|MulticastDetonate)
    (Default|CallServerMCOMDetonate self)
    (if _bvalid
      (Default|MCOMDestroyed _mcommanager (Getters|GetMCOMIndex) (Variables|Data-ServerArming|GetArmerRSHPRI)))))

(fn MCOMDisarm
  (if (Networking|IsServer)
    (Variables|DataReplicated|SetbArmed false)
    (CallFunction|MulticastDisarm)))

(fn OnRepBDetonated
  (bind _bdetonated (Variables|DataReplicated|GetbDetonated))
  (Development|SetHiddeninGame (Variables|Default|GetMCOM) _bdetonated true)
  (Development|SetHiddeninGame (Variables|Default|GetMGONE) (not _bdetonated) true))

(fn OnRepArmStartTime
  (if (!= (Variables|DataReplicated|GetArmStartTime) (.ArmTime (Utilities|GetClassDefaults "RSH_MCOM_C")))
    (Sounds|ArmedSounds)
    (else
      (Sounds|StopAllMCOMSounds))))

(fn GetDetonationTime
  (params (bGetPreIntenseTime :type Boolean))
  (if bGetPreIntenseTime
    (return (- (Variables|Config-RSH|GetDetonationTime) (Variables|/Script/Engine.SoundBase|GetDuration (Variables|/Script/Engine.AudioComponent|GetSound (Variables|Default|GetAudioArmedIntense)))))
    (else
      (return (Variables|Config-RSH|GetDetonationTime)))))

(fn GetArmedTime
  (return (- (GameState|GetServerWorldTimeSeconds (Game|GetGameState)) (Variables|DataReplicated|GetArmStartTime))))

(fn StopAllMCOMSounds
  (for _array_element (Actor|GetComponentsByClass "/Script/Engine.AudioComponent")
    (Audio|Components|Audio|Stop _array_element)))

(fn ArmedSounds
  (if (< (Getters|GetArmedTime) (Getters|GetDetonationTime true))
    (CallFunction|ArmedSoundTimer)
    (else
      (CallFunction|ArmedIntenseSoundTimer))))

(fn GetObjectiveName
  (bind (_mcommanager _bvalid) (CallFunction|GetMCOMManager))
  (bind _objectiveshortnames (Variables|/Game/CustomMaps/UGC1967262879/RSH/Blueprints/LevelActors/CORE/RSH_MCOMManager.RSH_MCOMManager_C|GetObjectiveShortNames _mcommanager))
  (if _bvalid
    (if (Utilities|Array|IsValidIndex _objectiveshortnames (Math|Conversions|ToInteger(Byte) (Variables|Config-RSH|GetMCOMIndex)))
      (return (Utilities|Array|Get(acopy) _objectiveshortnames (Math|Conversions|ToInteger(Byte) (Variables|Config-RSH|GetMCOMIndex))))
      (else
        (return "-1")))
    (else
      (return "-1"))))

(fn UpdateObjectiveWidget
  (bind _returnvalue (Transformation|GetActorLocation))
  (bind _asrsh_player_replication_info (Utilities|Casting|CastToRSH_PlayerReplicationInfo (CallFunction|GetLocalPRI)))
  (Development|SetHiddeninGame (Variables|Default|GetWidgetObjective) (Math|Boolean|ORBoolean (Default|GetIsinArmory _asrsh_player_replication_info) (not (Getters|IsActive)) (Getters|IsDetonated)) false)
  (if (not (Math|Boolean|ORBoolean (Default|GetIsinArmory _asrsh_player_replication_info) (not (Getters|IsActive)) (Getters|IsDetonated)))
    (if (.bIsValid (Default|GetPlayerPawn _asrsh_player_replication_info))
      (Transformation|SetWorldRotation (Variables|Default|GetWidgetObjective) (Math|Conversions|RotationFromXVector (CallFunction|GetDirtoFlat (Transformation|GetActorLocation (.Pawn (Default|GetPlayerPawn _asrsh_player_replication_info))) _returnvalue true)) false false)
      (Utilities|FlowControl|Sequence
        (:then_0
          (Transformation|SetRelativeLocation (Variables|Default|GetWidgetObjective) (Math|Vector|Lerp(Vector) (Variables|/Script/Engine.SceneComponent|GetRelativeLocation (Variables|Default|GetLowestPosition)) (Variables|/Script/Engine.SceneComponent|GetRelativeLocation (Variables|Default|GetHighestPosition)) (CallFunction|GetPctBetween (Math|Vector|VectorLength (CallFunction|GetDirto (Transformation|GetActorLocation (.Pawn (Default|GetPlayerPawn _asrsh_player_replication_info))) _returnvalue false)) (Variables|Config-Obj|GetMinObjWidgetDist) (Variables|Config-Obj|GetMaxObjWidgetDist) true)) false false))
        (:then_1
          (Transformation|SetRelativeScale3D (Variables|Default|GetWidgetObjective) (* (Math|Vector|MakeVector 1.0 1.0 1.0) (CallFunction|GetPctOf (CallFunction|GetPctBetween (Math|Vector|VectorLength (CallFunction|GetDirto (Transformation|GetActorLocation (.Pawn (Default|GetPlayerPawn _asrsh_player_replication_info))) _returnvalue false)) (Variables|Config-Obj|GetMinObjWidgetDist) (Variables|Config-Obj|GetMaxObjWidgetDist) true) (Variables|Config-Obj|GetMinObjWidgetScale) (Variables|Config-Obj|GetMaxObjWidgetScale)))))
        (:then_2
          (if (> (CallFunction|GetPctBetween (Math|Vector|VectorLength (CallFunction|GetDirto (Transformation|GetActorLocation (.Pawn (Default|GetPlayerPawn _asrsh_player_replication_info))) _returnvalue false)) (Variables|Config-Obj|GetMinObjWidgetDist) (Variables|Config-Obj|GetMaxObjWidgetDist) true) 0.0)
            (bind _aspmf_line_renderer (Utilities|Casting|CastToPMF_LineRenderer (Variables|/Script/Engine.ChildActorComponent|GetChildActor (Variables|Default|GetChildActorLineRenderer))))
            (Default|SetLineRenderer _aspmf_line_renderer (Transformation|GetWorldLocation (Variables|Default|GetWidgetObjectiveBelowOffset)) (Transformation|GetWorldLocation (Variables|Default|GetLowestPosition)) 0.05)))))))

(fn GetArmedPct
  (if (Variables|DataReplicated|GetbArmed)
    (if (Variables|DataReplicated|GetbDetonated)
      (return 1.0)
      (else
        (return (Math|Float|Clamp(Float) (/ (Getters|GetArmedTime) (Getters|GetDetonationTime false))))))
    (else
      (return 0.0))))

(fn SetupWidget
  (bind _asrsh_ui_world_objective (Utilities|Casting|CastToRSH_UI_World_Objective (UserInterface|GetUserWidgetObject (Variables|Default|GetWidgetObjective))))
  (Variables|/Game/CustomMaps/UGC1967262879/RSH/Blueprints/UMG/RSH_UI_World_Objective.RSH_UI_World_Objective_C|SetOwningMCOM _asrsh_ui_world_objective self))

(fn TrackLocalArming
  (bind _localarmerrshpri (Variables|Data-LocalArming|GetLocalArmerRSHPRI))
  (bind (_character _bisvalid) (Default|GetPlayerCharacter _localarmerrshpri))
  (if (Math|Boolean|ANDBoolean (not (Variables|DataReplicated|GetbArmed)) (not (Variables|DataReplicated|GetbDetonated)) (Variables|DataReplicated|GetbIsActive) (Getters|IsLocalArming))
    (bind _bcanarm (LocalArming|CanDoLocalArming (Variables|Data-LocalArming|GetLocalArmerRSHPRI)))
    (if _bcanarm
      (if _bisvalid
        (if (not (< (Transformation|GetDistanceTo _character self) (Variables|Config-RSH|GetMaxArmingDistance)))
          (LocalArming|CancelLocalArming true))
        (else
          (LocalArming|CancelLocalArming false)))
      (else
        (LocalArming|CancelLocalArming false)))))

(fn IsArmed
  (return (Variables|DataReplicated|GetbArmed)))

(fn IsDetonated
  (return (Variables|DataReplicated|GetbDetonated)))

(fn IsActive
  (return (Variables|DataReplicated|GetbIsActive)))

(fn SetActive
  (params (bNewIsActive :type Boolean))
  (if (Variables|DataReplicated|GetbDetonated)
    (if (not bNewIsActive) ; You can't activate that of which is destroyed
      (Variables|DataReplicated|SetbIsActive false))
    (else
      (Variables|DataReplicated|SetbIsActive bNewIsActive))))

(fn FullMCOMRestore
  (Variables|DataReplicated|SetbIsActive false)
  (Variables|DataReplicated|SetbDetonated false)
  (Variables|DataReplicated|SetbArmed false)
  (Variables|Data-ServerArming|SetArmerRSHPRI 0))

(fn StartLocalDisarming
  (params (RSHPRI :type RSH%20Player%20Replication%20Info%20Object%20Reference))
  (bind _bcanarm (LocalDisarming|CanDoLocalDisarming RSHPRI))
  (if _bcanarm
    (bind _output_get (Variables|Data-LocalDisarming|SetLocalDisarmerRSHPRI RSHPRI))
    (Audio|Components|Audio|Play (Variables|Default|GetAudioDisarming) 0.0)
    (CallFunction|DisarmingTimer)
    (CallFunction|AddPMFLog (Utilities|String|Append "Local Disarm Start! IsValid: " (Utilities|String|ToString(Boolean) (Utilities|IsValid _output_get))))
    (else
      (CallFunction|AddPMFLog "Start Local Disarming() Could not arm"))))

(fn RestoreMCOM
  (Variables|DataReplicated|SetbArmed false)
  (Variables|DataReplicated|SetbIsActive false)
  (Variables|DataReplicated|SetbDetonated false))

(fn CanDoLocalDisarming
  (params (RSHPRI :type RSH%20Player%20Replication%20Info%20Object%20Reference))
  (Utilities|IsValid RSHPRI
    (:Is%20Valid
      (if (not (Default|IsDead RSHPRI))
        (return true)
        (else
          (return false))))
    (:Is%20Not%20Valid
      (return false))))

(fn TrackLocalDisarming
  (bind _localdisarmerrshpri (Variables|Data-LocalDisarming|GetLocalDisarmerRSHPRI))
  (bind (_character _bisvalid) (Default|GetPlayerCharacter _localdisarmerrshpri))
  (if (Math|Boolean|ANDBoolean (Variables|DataReplicated|GetbArmed) (not (Variables|DataReplicated|GetbDetonated)) (Variables|DataReplicated|GetbIsActive) (Getters|IsLocalDisarming))
    (bind _bcanarm (LocalDisarming|CanDoLocalDisarming (Variables|Data-LocalDisarming|GetLocalDisarmerRSHPRI)))
    (if _bcanarm
      (if _bisvalid
        (if (not (< (Transformation|GetDistanceTo _character self) (Variables|Config-RSH|GetMaxDisarmingDistance)))
          (LocalDisarming|CancelLocalDisarming true))
        (else
          (LocalDisarming|CancelLocalDisarming false)))
      (else
        (LocalDisarming|CancelLocalDisarming false)))))

(fn CancelLocalDisarming
  (params (bWasCanceledByPlayer :type Boolean))
  (Utilities|FlowControl|Sequence
    (:then_0
      (Audio|Components|Audio|Stop (Variables|Default|GetAudioDisarming))
      (Variables|Data-LocalDisarming|SetLocalDisarmerRSHPRI 0)
      (Cable|StopCableVisual))
    (:then_1
      (if bWasCanceledByPlayer
        (Audio|PlaySoundatLocation "/Game/CustomMaps/UGC1967262879/PMF/Audio/WINDOWS_XP_ERROR_SOUND.WINDOWS_XP_ERROR_SOUND" (Transformation|GetActorLocation) "0, 0, 0" 1.0 1.0 0.0 0 0 0)
        (CallFunction|AddPMFConstantLog "CancelLocalDisarming" "By Player")
        (else
          (CallFunction|AddPMFConstantLog "CancelLocalDisarming" "Not By Player"))))))

(fn IsLocalDisarming
  (return (Utilities|IsValid (Variables|Data-LocalDisarming|GetLocalDisarmerRSHPRI))))

(fn IsLocalArming
  (return (Utilities|IsValid (Variables|Data-LocalArming|GetLocalArmerRSHPRI))))

(fn FinishLocalDisarming
  (Cable|StopCableVisual)
  (Utilities|IsValid (Variables|Data-LocalDisarming|GetLocalDisarmerRSHPRI)
    (:Is%20Valid
      (Default|DisarmMCOM (Variables|Data-LocalDisarming|GetLocalDisarmerRSHPRI) (Getters|GetMCOMIndex))
      (Variables|Data-LocalDisarming|SetLocalDisarmerRSHPRI 0))
    (:Is%20Not%20Valid
      (CallFunction|AddPMFLog "Finish Local Disarming Not Valid RSHPRI"))))

(fn StartCableVisual
  (params (HandActor :type Actor%20Object%20Reference))
  (Components|Activation|Activate (Variables|Default|GetCable_L) true)
  (Class|CableComponent|SetAttachEndto (Variables|Default|GetCable_L) HandActor "None" "None")
  (Development|SetHiddeninGame (Variables|Default|GetCable_L) false false))

(fn StopCableVisual
  (Class|CableComponent|SetAttachEndto (Variables|Default|GetCable_L) 0 "None" "None")
  (Development|SetHiddeninGame (Variables|Default|GetCable_L) true false)
  (Components|Activation|Deactivate (Variables|Default|GetCable_R)))

(fn UpdateArmedLight)

(fn GetInteractionMessage
  (params (UserPRI :type PMF%20Player%20Replication%20Info%20Object%20Reference) (UserCPI :type PMF%20Character%20Proxy%20Info%20Object%20Reference) (UserCustomHand :type PMF%20Custom%20Hand%20Object%20Reference))
  (bind _bisinteractable (CallFunction|IsInteractable UserPRI UserCPI UserCustomHand))
  (if _bisinteractable
    (Utilities|IsValid UserPRI
      (:Is%20Valid
        (bind _asrsh_player_replication_info (Utilities|Casting|CastToRSH_PlayerReplicationInfo UserPRI)
          (:then
            (return (select (Default|IsAttacker _asrsh_player_replication_info) "Plant Bomb" "Defuse Bomb")))
          (:CastFailed
            (return ""))))
      (:Is%20Not%20Valid
        (return "")))))

(fn IsInteractable
  (params (UserPRI :type PMF%20Player%20Replication%20Info%20Object%20Reference) (UserCPI :type PMF%20Character%20Proxy%20Info%20Object%20Reference) (UserCustomHand :type PMF%20Custom%20Hand%20Object%20Reference))
  (if (and (not (Variables|DataReplicated|GetbDetonated)) (Variables|DataReplicated|GetbIsActive))
    (bind _asrsh_player_replication_info (Utilities|Casting|CastToRSH_PlayerReplicationInfo UserPRI)
      (:then
        (if (Default|IsAttacker _asrsh_player_replication_info)
          (return (and (not (Variables|DataReplicated|GetbArmed)) (not (Getters|IsLocalArming))))
          (else
            (bind _asrsh_game_logic (Utilities|Casting|CastToRSH_GameLogic (CallFunction|GetPMFGameLogic))
              (:then
                (if (Variables|/Game/CustomMaps/UGC1967262879/RSH/Blueprints/LevelActors/CORE/RSH_GameLogic.RSH_GameLogic_C|GetbRestrictPlantingToSpecificRoles _asrsh_game_logic)
                  (if (.bIsValid (Default|GetRSHRole _asrsh_player_replication_info))
                    (return (and (Utilities|Struct|BreakRSH_RoleInfo (.RSHRoleInfo (Default|GetRSHRole _asrsh_player_replication_info))) (Getters|IsArmed)))
                    (else
                      _))))
              (:CastFailed
                _))
            (return (Getters|IsArmed)))))
      (:CastFailed
        (return false)))
    (else
      (return false))))