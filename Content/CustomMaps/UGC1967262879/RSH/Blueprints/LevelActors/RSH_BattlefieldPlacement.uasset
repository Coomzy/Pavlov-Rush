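; RSH_BattlefieldPlacement is a level actor that marks a battlefield placement point and carries an active flag.
; Its Capsule component supplies the world location returned by GetPlacementLoc.
; GetIsActive reads the IsActive flag, and SetIsActive changes it only on the server.
; The construction script is empty, and the actor holds no placement logic of its own.
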(fn ConstructionScript)

(fn GetPlacementLoc
  (return (Transformation|GetWorldLocation (Variables|Default|GetCapsule))))

(fn GetIsActive
  (return (Variables|Status|GetbIsActive)))

(fn SetIsActive
  (params (NewIsActive :type Boolean))
  (if (Networking|IsServer)
    (Variables|Status|SetbIsActive NewIsActive)))