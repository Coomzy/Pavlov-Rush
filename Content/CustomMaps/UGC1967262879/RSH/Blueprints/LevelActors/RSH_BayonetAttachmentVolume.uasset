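; RSH bayonet attachment volume, a level actor that gives eligible items entering its box a bayonet attachment.
; On server-side overlap, it resolves the actor's class to an item ID and asks RSH_GameLogic whether that item can take a bayonet.
; Eligible items without an attached RSH_BayoAttachment get one spawned with the item as owner, passing the socket and offsets from the returned bayonet info.
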(event OnComponentBeginOverlap(Box)
  (params (OverlappedComponent :type Primitive%20Component%20Object%20Reference) (OtherActor :type Actor%20Object%20Reference) (OtherComp :type Primitive%20Component%20Object%20Reference) (OtherBodyIndex :type Integer) (bFromSweep :type Boolean) (SweepResult :type Hit%20Result%20Structure%20%28by%20ref%29))
  (if (Networking|IsServer)
    (bind _itemid (CallFunction|GetItemIDbyClass (Utilities|GetClass OtherActor)))
    (if (Utilities|Enum|NotEqual(Enum) _itemid "NewEnumerator42")
      (bind _asrsh_game_logic (Utilities|Casting|CastToRSH_GameLogic (CallFunction|GetPMFGameLogic)))
      (bind (_bcanhavebayo _bayoinfo) (Default|CanItemHaveBayo _asrsh_game_logic _itemid))
      (if _bcanhavebayo
        (CallFunction|TrySpawnBayoforItem OtherActor _bayoinfo)))))

(event EventBeginPlay)

(event Collision|EventActorBeginOverlap
  (params (OtherActor :type Actor%20Object%20Reference)))

(event EventTick
  (params (DeltaSeconds :type Float%20%28single-precision%29)))

(fn ConstructionScript)

(fn TrySpawnBayoforItem
  (params (ItemActor :type Actor%20Object%20Reference) (BayoInfo :type RSH%20Bayo%20Info%20Structure))
  (bind (_itemid _sockettoattach _bayooffset _bayorotoffset) (Utilities|Struct|BreakRSH_BayoInfo BayoInfo))
  (if (Networking|IsServer)
    (Utilities|IsValid ItemActor
      (:Is%20Valid
        (bind _bhasbayo (CallFunction|DoesItemAlreadyHaveBayo ItemActor))
        (if (not _bhasbayo)
          (Game|SpawnActorfromClass (Variables|Config|GetBayoAttachmentClass) (Math|Transform|MakeTransform "0, 0, 0") "AlwaysSpawn" ItemActor _bayooffset _bayorotoffset ItemActor _sockettoattach 0))))))

(fn DoesItemAlreadyHaveBayo
  (params (ItemActor :type Actor%20Object%20Reference))
  (Utilities|IsValid ItemActor
    (:Is%20Valid
      (for _array_element (Actor|GetAttachedActors ItemActor)
        (Utilities|Casting|CastToRSH_BayoAttachment _array_element)
        (return true))
      (return false))
    (:Is%20Not%20Valid
      (return true))))