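; RSH level actor that teleports an entering player's character to its TeleportPoint and assigns its configured RoleIndex through the player's replication info.
; CheckForErrors looks up RSH_GameLogic's role list for the TeamType, prints validation results and sets RoleText to the role name.
; It also flags a missing game logic or TeleportPoint.
; As wired, the role lookup runs only when RoleIndex equals 255; other values print the default-index error.
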(event EventOnPlayerEnter
  (params (PRI :type PMF%20Player%20Replication%20Info%20Object%20Reference) (Pawn :type Pawn%20Object%20Reference))
  (bind _ascharacter (Utilities|Casting|CastToCharacter Pawn))
  (Transformation|SetActorLocation _ascharacter (Transformation|GetActorLocation (Variables|Default|GetTeleportPoint)) false true)
  (bind _asrsh_player_replication_info (Utilities|Casting|CastToRSH_PlayerReplicationInfo PRI))
  (Default|ServerSetRoleIndex _asrsh_player_replication_info (Variables|Config|GetRoleIndex)))

(fn ConstructionScript
  (|CallParentFunction))

(fn CheckforErrors
  (bind _roleindex (Variables|Config|GetRoleIndex))
  (Utilities|FlowControl|Sequence
    (:then_0
      (bind _outactors (Actor|GetAllActorsOfClass "/Game/CustomMaps/UGC1967262879/RSH/Blueprints/LevelActors/CORE/RSH_GameLogic.RSH_GameLogic_C"))
      (Utilities|IsValid (Utilities|Array|Get(acopy) _outactors)
        (:Is%20Valid
          (if (== (Variables|Config|GetRoleIndex) 255)
            (if (< (Math|Conversions|ToInteger(Byte) (Variables|Config|GetRoleIndex)) (Utilities|Array|Length (Utilities|Select :Index (Variables|Config|GetTeamType) :NewEnumerator0 (Default|GetAttackersTeamRoles (Utilities|Array|Get(acopy) _outactors)) :NewEnumerator1 (Default|GetDefendersTeamRoles (Utilities|Array|Get(acopy) _outactors)))))
              (Development|PrintString (Utilities|String|Append "RoleIndex is '" (Utilities|String|ToString(Byte) _roleindex) "' and is assigned to Role '" (.RoleName (Utilities|Struct|BreakRSH_RoleInfo (Utilities|Array|Get(acopy) (Utilities|Select :Index (Variables|Config|GetTeamType) :NewEnumerator0 (Default|GetAttackersTeamRoles (Utilities|Array|Get(acopy) _outactors)) :NewEnumerator1 (Default|GetDefendersTeamRoles (Utilities|Array|Get(acopy) _outactors))) (Math|Conversions|ToInteger(Byte) _roleindex)))) "'") true true "(R=0.038389,G=1.000000,B=0.194267,A=1.000000)" 5.0)
              (Rendering|Components|TextRender|SetText (Variables|Default|GetRoleText) (Utilities|Text|ToText(String) (.RoleName (Utilities|Struct|BreakRSH_RoleInfo (Utilities|Array|Get(acopy) (Utilities|Select :Index (Variables|Config|GetTeamType) :NewEnumerator0 (Default|GetAttackersTeamRoles (Utilities|Array|Get(acopy) _outactors)) :NewEnumerator1 (Default|GetDefendersTeamRoles (Utilities|Array|Get(acopy) _outactors))) (Math|Conversions|ToInteger(Byte) _roleindex))))))
              (else
                (Development|PrintString (Utilities|String|Append "ERROR: RoleIndex is great than amount of Roles, Amount Of Roles = " (Utilities|String|ToString(Integer) (Utilities|Array|Length (Utilities|Select :Index (Variables|Config|GetTeamType) :NewEnumerator0 (Default|GetAttackersTeamRoles (Utilities|Array|Get(acopy) _outactors)) :NewEnumerator1 (Default|GetDefendersTeamRoles (Utilities|Array|Get(acopy) _outactors))))) ", RoleIndex = " (Utilities|String|ToString(Byte) (Variables|Config|GetRoleIndex))) true true "(R=1.000000,G=0.006821,B=0.000000,A=1.000000)" 5.0)))
            (else
              (Development|PrintString "ERROR: RoleIndex is default at 255!" true true "(R=1.000000,G=0.000000,B=0.060741,A=1.000000)" 5.0))))
        (:Is%20Not%20Valid
          (Development|PrintString "ERROR: No RSH_GameLogic!" true true "(R=1.000000,G=0.000000,B=0.051918,A=1.000000)" 5.0))))
    (:then_1
      (Utilities|IsValid (Variables|Default|GetTeleportPoint)
        (:Is%20Not%20Valid
          (Development|PrintString "ERROR: No TeleportPoint!" true true "(R=1.000000,G=0.000000,B=0.051918,A=1.000000)" 5.0))))))