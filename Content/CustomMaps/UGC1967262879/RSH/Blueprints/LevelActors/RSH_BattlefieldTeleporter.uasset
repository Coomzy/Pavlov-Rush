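; RSH teleporter level actor that sends an entering player to the battlefield on their team's side.
; On player enter, it calls GoToBattlefield on the player's RSH_PlayerReplicationInfo.
; It then picks from the MCOM manager's defender or attacker battlefield placements at random and sets the client's location and yaw from them.
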(event EventOnPlayerEnter
  (params (PRI :type PMF%20Player%20Replication%20Info%20Object%20Reference) (Pawn :type Pawn%20Object%20Reference))
  (bind _mcommanager (CallFunction|GetMCOMManager))
  (Utilities|FlowControl|Sequence
    (:then_0
      (bind _asrsh_player_replication_info (Utilities|Casting|CastToRSH_PlayerReplicationInfo PRI))
      (Default|GotoBattlefield _asrsh_player_replication_info))
    (:then_1
      (bind _asrsh_player_replication_info_2 (Utilities|Casting|CastToRSH_PlayerReplicationInfo PRI))
      (Default|ClientSetLocandRot PRI (Transformation|GetActorLocation (Utilities|Array|Get(acopy) (select (Default|IsDefender _asrsh_player_replication_info_2) (Variables|/Game/CustomMaps/UGC1967262879/RSH/Blueprints/LevelActors/CORE/RSH_MCOMManager.RSH_MCOMManager_C|GetDefendersBattlefieldPlacements _mcommanager) (Variables|/Game/CustomMaps/UGC1967262879/RSH/Blueprints/LevelActors/CORE/RSH_MCOMManager.RSH_MCOMManager_C|GetAttackersBattlefieldPlacements _mcommanager)) (Math|Random|RandomIntegerinRange 0 (- (Utilities|Array|Length (select (Default|IsDefender _asrsh_player_replication_info_2) (Variables|/Game/CustomMaps/UGC1967262879/RSH/Blueprints/LevelActors/CORE/RSH_MCOMManager.RSH_MCOMManager_C|GetDefendersBattlefieldPlacements _mcommanager) (Variables|/Game/CustomMaps/UGC1967262879/RSH/Blueprints/LevelActors/CORE/RSH_MCOMManager.RSH_MCOMManager_C|GetAttackersBattlefieldPlacements _mcommanager))) 1)))) (.Yaw (Math|Rotator|BreakRotator (Transformation|GetActorRotation (Utilities|Array|Get(acopy) (select (Default|IsDefender _asrsh_player_replication_info_2) (Variables|/Game/CustomMaps/UGC1967262879/RSH/Blueprints/LevelActors/CORE/RSH_MCOMManager.RSH_MCOMManager_C|GetDefendersBattlefieldPlacements _mcommanager) (Variables|/Game/CustomMaps/UGC1967262879/RSH/Blueprints/LevelActors/CORE/RSH_MCOMManager.RSH_MCOMManager_C|GetAttackersBattlefieldPlacements _mcommanager)) (Math|Random|RandomIntegerinRange 0 (- (Utilities|Array|Length (select (Default|IsDefender _asrsh_player_replication_info_2) (Variables|/Game/CustomMaps/UGC1967262879/RSH/Blueprints/LevelActors/CORE/RSH_MCOMManager.RSH_MCOMManager_C|GetDefendersBattlefieldPlacements _mcommanager) (Variables|/Game/CustomMaps/UGC1967262879/RSH/Blueprints/LevelActors/CORE/RSH_MCOMManager.RSH_MCOMManager_C|GetAttackersBattlefieldPlacements _mcommanager))) 1))))))))))

(fn ConstructionScript
  (|CallParentFunction))