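; Return-to-battlefield volume for RSH maps that flags players of the affected team (attackers, defenders or both) as out of bounds while inside it.
; The server sets a replicated enabled state, which AlwaysActive forces on.
; Enter and exit events notify only the local player's replication info.
; On clients, OnRep rechecks overlapping characters when the state toggles, so a player already inside is flagged or cleared.
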(event EventBeginPlay
  (|CallParentFunction)
  (if (Networking|IsServer)
    (if (Variables|Config|GetbAlwaysActive)
      (Setters|SetIsEnabled true))))

(event EventOnPlayerEnter
  (params (PRI :type PMF%20Player%20Replication%20Info%20Object%20Reference) (Pawn :type Pawn%20Object%20Reference))
  (if (Getters|GetIsEnabled)
    (bind _asrsh_player_replication_info (Utilities|Casting|CastToRSH_PlayerReplicationInfo PRI))
    (bind _bboundsapplytoplayer (Info|DoBoundsApplytoPlayer _asrsh_player_replication_info))
    (if _bboundsapplytoplayer
      (Default|PlayerHasGoneOutOfBounds _asrsh_player_replication_info self))))

(event EventOnPlayerExit
  (params (PRi :type PMF%20Player%20Replication%20Info%20Object%20Reference) (Pawn :type Pawn%20Object%20Reference))
  (if (Getters|GetIsEnabled)
    (bind _asrsh_player_replication_info (Utilities|Casting|CastToRSH_PlayerReplicationInfo PRi))
    (bind _bboundsapplytoplayer (Info|DoBoundsApplytoPlayer _asrsh_player_replication_info))
    (if _bboundsapplytoplayer
      (Default|PlayerHasReturnedfromOutOfBounds _asrsh_player_replication_info self))))

(fn ConstructionScript
  (|CallParentFunction))

(fn DoBoundsApplytoPlayer
  (params (RSHPRI :type RSH%20Player%20Replication%20Info%20Object%20Reference))
  (Utilities|IsValid RSHPRI
    (:Is%20Valid
      (if (Default|IsLocalPRI RSHPRI)
        (switch Utilities|FlowControl|Switch|SwitchonERSH_TeamSelection (Variables|Config|GetTeamEffected)
          (:NewEnumerator2
            (return true))
          (:NewEnumerator0
            (return (Default|IsAttacker RSHPRI)))
          (:NewEnumerator1
            (return (Default|IsDefender RSHPRI))))
        (else
          _)))
    (:Is%20Not%20Valid
      _))
  (return false))

(fn SetIsEnabled
  (params (bNewIsEnabled :type Boolean))
  (if (Networking|IsServer)
    (if (Variables|Config|GetbAlwaysActive)
      (Variables|DataReplicated|SetbIsEnabled true)
      (else
        (Variables|DataReplicated|SetbIsEnabled bNewIsEnabled)))))

(fn GetIsEnabled
  (return (Variables|DataReplicated|GetbIsEnabled)))

(fn OnRepBIsEnabled
  (if (not (Networking|IsServer)) ; This is all managed client side
    (if (Variables|DataReplicated|GetbIsEnabled)
      (EnabledEvents|OnBoundsEnabled)
      (else
        (EnabledEvents|OnBoundsDisabled)))))

(fn OnBoundsDisabled
  (for _array_element (Collision|GetOverlappingActors (Variables|Default|GetPlayerCollisionBox) "/Script/Engine.Character" :!class /Script/Engine.PrimitiveComponent)
    (bind _ascharacter (Utilities|Casting|CastToCharacter _array_element))
    (if (Pawn|IsLocallyControlled _ascharacter)
      (bind (_outpri _bvalid) (Default|GetPRIbyPlayerState (CallFunction|GetPMFGameLogic) (Variables|/Script/Engine.Pawn|GetPlayerState _ascharacter)))
      (if _bvalid
        (bind _asrsh_player_replication_info (Utilities|Casting|CastToRSH_PlayerReplicationInfo _outpri))
        (bind _bboundsapplytoplayer (Info|DoBoundsApplytoPlayer _asrsh_player_replication_info))
        (if _bboundsapplytoplayer
          (Default|PlayerHasReturnedfromOutOfBounds _asrsh_player_replication_info self)
          (return) ; There is only ONE local player, \nif we've made it this far we've done our job
        )))))

(fn OnBoundsEnabled
  (for _array_element (Collision|GetOverlappingActors (Variables|Default|GetPlayerCollisionBox) "/Script/Engine.Character" :!class /Script/Engine.PrimitiveComponent)
    (bind _ascharacter (Utilities|Casting|CastToCharacter _array_element))
    (if (Pawn|IsLocallyControlled _ascharacter)
      (bind (_outpri _bvalid) (Default|GetPRIbyPlayerState (CallFunction|GetPMFGameLogic) (Variables|/Script/Engine.Pawn|GetPlayerState _ascharacter)))
      (if _bvalid
        (bind _asrsh_player_replication_info (Utilities|Casting|CastToRSH_PlayerReplicationInfo _outpri))
        (bind _bboundsapplytoplayer (Info|DoBoundsApplytoPlayer _asrsh_player_replication_info))
        (if _bboundsapplytoplayer
          (Default|PlayerHasGoneOutOfBounds _asrsh_player_replication_info self)
          (return) ; There is only ONE local player, \nif we've made it this far we've done our job
        )))))