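; RSH round-over screen actor, shown on the owning player's VR pawn while the round state is Ended.
; It snaps onto that pawn on spawn and re-checks every tick, reattaching if the pawn changes.
; Shortly after spawn it can optionally take the headset camera's relative yaw as its initial rotation.
; It destroys itself once the game logic's round state is no longer Ended.
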(event Custom|AttachToPawn
  (bind _owningpri (Variables|Default|GetOwningPRI))
  (bind _pawn (Default|GetPlayerPawn _owningpri))
  (Utilities|IsValid (Variables|Default|GetOwningPRI)
    (:Is%20Valid
      (bind _aspawn (Utilities|Casting|CastToPawn (Actor|GetAttachParentActor))
        (:then
          (if (!= _aspawn _pawn)
            (Transformation|AttachActorToActor _pawn "None" "SnapToTarget" "SnapToTarget" "KeepRelative" true :!label _label)))
        (:CastFailed
          (goto _label))))))

(event EventBeginPlay
  (bind _owningpri (Variables|Default|GetOwningPRI))
  (bind _vrcamera (Default|GetVRHeadsetCamera _owningpri))
  (|CallParentFunction)
  (CallFunction|AttachtoPawn)
  (Utilities|FlowControl|Delay 0.2) ; Wait for it...
  (if (Variables|Default|GetbSetInitalRotationToCameraDir)
    (Utilities|IsValid _vrcamera
      (:Is%20Valid
        (Transformation|SetActorRelativeRotation (Math|Rotator|MakeRotator 0.0 0.0 (.Yaw (Math|Rotator|BreakRotator (Variables|/Script/Engine.SceneComponent|GetRelativeRotation _vrcamera)))))))))

(event EventTick
  (params (DeltaSeconds :type Float%20%28single-precision%29))
  (|CallParentFunction DeltaSeconds)
  (if (Utilities|Enum|NotEqual(Enum) (Variables|/Game/CustomMaps/UGC1967262879/PMF/Blueprints/LevelActors/CORE/PMF_GameLogic.PMF_GameLogic_C|GetCurRoundState (CallFunction|GetPMFGameLogic)) "Ended")
    (Actor|DestroyActor)
    (else
      (CallFunction|AttachtoPawn))))

(fn ConstructionScript)