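; Bayonet attachment that snaps to a socket on its weapon item server-side and destroys itself when that item is gone.
; The holder is resolved through the attachment chain; their local client detects box overlaps, plays the stab sound and registers hits via RSH PRI.
; Its team check compares the holder's PRI to itself, not the victim's.
; ServerGetBayoHit applies damage and multicasts the sound, skipped for the local holder.
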(event OnComponentBeginOverlap(Box)
  (params (OverlappedComponent :type Primitive%20Component%20Object%20Reference) (OtherActor :type Actor%20Object%20Reference) (OtherComp :type Primitive%20Component%20Object%20Reference) (OtherBodyIndex :type Integer) (bFromSweep :type Boolean) (SweepResult :type Hit%20Result%20Structure%20%28by%20ref%29))
  (bind (_rshpri _bisvalid) (CallFunction|GetHoldingOwner))
  (bind _character (Default|GetPlayerCharacter _rshpri))
  (if _bisvalid
    (if (Default|IsLocalPRI _rshpri)
      (bind _ascharacter (Utilities|Casting|CastToCharacter OtherActor))
      (if (!= _ascharacter _character)
        (bind (_outpri _bvalid) (Default|GetPRIbyPlayerState (CallFunction|GetPMFGameLogic) (Variables|/Script/Engine.Pawn|GetPlayerState _character)))
        (if _bvalid
          (if (!= (Default|GetTeamIndex _outpri) (Default|GetTeamIndex _rshpri))
            (Default|RegisterBayoHit _rshpri _ascharacter self)
            (Audio|PlaySoundatLocation (Variables|Default|GetStabSound) (Transformation|GetActorLocation) "0, 0, 0" 1.0 1.0 0.0 0 0 0)))))))

(event Custom|MulticastPlayStabSound
  (if (not (Default|IsLocalPRI (.RSHPRI (CallFunction|GetHoldingOwner))))
    (Audio|PlaySoundatLocation (Variables|Default|GetStabSound) (Transformation|GetActorLocation) "0, 0, 0" 1.0 1.0 0.0 0 0 0)))

(event EventBeginPlay
  (|CallParentFunction)
  (if (Networking|IsServer)
    (Transformation|AttachActorToActor (Variables|DataReplicated|GetItemActor) (Variables|Setup|GetSocket) "SnapToTarget" "SnapToTarget" "SnapToTarget" true)
    (Transformation|SetRelativeLocationAndRotation (Variables|Default|GetDefaultSceneRoot) (Variables|Setup|GetOffsetVector) (Variables|Setup|GetOffsetRotator) false false)))

(event EventTick
  (params (DeltaSeconds :type Float%20%28single-precision%29))
  (|CallParentFunction DeltaSeconds)
  (if (Networking|IsServer)
    (Utilities|IsValid (Variables|DataReplicated|GetItemActor)
      (:Is%20Not%20Valid
        (Actor|DestroyActor)))))

(fn ConstructionScript)

(fn GetHoldingOwner
  (bind _itemactor (Variables|DataReplicated|GetItemActor))
  (bind _returnvalue (Actor|GetAttachParentActor _itemactor))
  (bind _returnvalue_2 (Actor|GetAttachParentActor _returnvalue))
  (Utilities|IsValid _itemactor
    (:Is%20Valid
      (Utilities|IsValid _returnvalue
        (:Is%20Valid
          (Utilities|IsValid _returnvalue_2
            (:Is%20Valid
              (bind _ascharacter (Utilities|Casting|CastToCharacter _returnvalue_2)
                (:then
                  (bind _outpri (Default|GetPRIbyPlayerState (CallFunction|GetPMFGameLogic) (Variables|/Script/Engine.Pawn|GetPlayerState _ascharacter)))
                  (bind _asrsh_player_replication_info (Utilities|Casting|CastToRSH_PlayerReplicationInfo _outpri)
                    (:then
                      (return _asrsh_player_replication_info true))
                    (:CastFailed
                      (return 0 false))))
                (:CastFailed
                  (return 0 false))))
            (:Is%20Not%20Valid
              (return 0 false))))
        (:Is%20Not%20Valid
          (return 0 false))))
    (:Is%20Not%20Valid
      (return 0 false))))

(fn ServerGetBayoHit
  (params (HitChar :type Character%20Object%20Reference) (HitterPRI :type RSH%20Player%20Replication%20Info%20Object%20Reference))
  (Utilities|IsValid HitChar
    (:Is%20Valid
      (Game|Damage|ApplyDamage HitChar (Variables|Default|GetBayoDamage) (Default|GetPlayerController HitterPRI) self "/Engine/EngineDamageTypes/DmgTypeBP_Environmental.DmgTypeBP_Environmental_C")
      (CallFunction|MulticastPlayStabSound))))