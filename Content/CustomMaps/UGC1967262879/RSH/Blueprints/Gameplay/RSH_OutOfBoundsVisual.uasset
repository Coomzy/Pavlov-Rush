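; An actor that displays an out-of-bounds visual on its OutOfBounds component and can show or hide it.
; It creates a dynamic material instance from the component's first material once, guarded by a flag.
; Scalar parameters for fade opacity, Fresnel power and overall opacity are then set on that instance.
; Editor helper functions toggle the visual and push editor-set values into the material for previewing.
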(fn ConstructionScript)

(fn EnableOutOfBoundsVisual
  (params (bEnable :type Boolean))
  (Rendering|SetVisibility (Variables|Default|GetOutOfBounds) bEnable true))

(fn CreateDynamicMaterialInstance
  (bind _outofbounds (Variables|Default|GetOutOfBounds))
  (if (not (Variables|Default|GetbHasCreatedDynamicMaterialInstance))
    (Variables|Default|SetbHasCreatedDynamicMaterialInstance true)
    (bind _returnvalue (Rendering|Material|CreateDynamicMaterialInstance _outofbounds 0 (Rendering|Material|GetMaterial _outofbounds 0) "None" :!class /Script/Engine.PrimitiveComponent))
    (bind _output_get (Variables|Default|SetDynamicMaterialInstance _returnvalue))
    (Rendering|Material|SetMaterial (Variables|Default|GetOutOfBounds) 0 _output_get)))

(fn SetDynamicMaterialInstanceValues
  (params (FadeOpacity :type Float%20%28single-precision%29) (FrenselPower :type Float%20%28single-precision%29) (OverallOpacity :type Float%20%28single-precision%29))
  (if (Variables|Default|GetbHasCreatedDynamicMaterialInstance)
    (Utilities|IsValid (Variables|Default|GetDynamicMaterialInstance)
      (:Is%20Valid
        (Rendering|Material|SetScalarParameterValue (Variables|Default|GetDynamicMaterialInstance) (Variables|Default|GetParamName_FadeOpacity) FadeOpacity :!class /Script/Engine.MaterialInstanceDynamic)
        (Rendering|Material|SetScalarParameterValue (Variables|Default|GetDynamicMaterialInstance) (Variables|Default|GetParamName_FrenselPower) FrenselPower :!class /Script/Engine.MaterialInstanceDynamic)
        (Rendering|Material|SetScalarParameterValue (Variables|Default|GetDynamicMaterialInstance) (Variables|Default|GetParamName_OverallOpacity) OverallOpacity :!class /Script/Engine.MaterialInstanceDynamic)))))

(fn EnableVisualEditor
  (CallFunction|EnableOutOfBoundsVisual true))

(fn DisableVisualEditor
  (CallFunction|EnableOutOfBoundsVisual false))

(fn UpdateDynamicMaterialInstanceValues
  (CallFunction|SetDynamicMaterialInstanceValues (Variables|Default|GetFadeOpacityEdtiorValue) (Variables|Default|GetFenselPowerEdtiorValue) (Variables|Default|GetOverallOpacityEdtiorValue)))