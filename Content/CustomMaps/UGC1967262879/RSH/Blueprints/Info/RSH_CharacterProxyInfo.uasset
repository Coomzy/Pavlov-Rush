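; RSH character proxy info that gives its owning character an out-of-bounds visual effect.
; On BeginPlay it spawns an actor of the configured visual class and snaps it to the character's CameraComponent.
; It exposes a getter and a validity-checked toggle for that visual, and switches it off in the player-died replication callback.
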(event EventBeginPlay
  (|CallParentFunction)
  (OutOfBoundsVisual|SpawnOutOfBoundsVisual))

(event EventOnRepPlayerDied
  (|CallParentFunction)
  (OutOfBoundsVisual|EnableOutOfBoundsVisual false))

(fn ConstructionScript
  (|CallParentFunction))

(fn SpawnOutOfBoundsVisual
  (bind _returnvalue (Game|SpawnActorfromClass (Variables|Config|GetOutOfBoundsVisualClass) (Math|Transform|MakeTransform "0, 0, 0") "AlwaysSpawn" 0 0))
  (bind _output_get (Variables|Data|SetOutOfBoundsVisual _returnvalue))
  (Transformation|AttachComponentToComponent _output_get (Actor|GetComponentbyClass (.OwningCharacter (CallFunction|GetOwningCharacter)) "/Script/Engine.CameraComponent") "None" "SnapToTarget" "SnapToTarget" "SnapToTarget" true))

(fn EnableOutOfBoundsVisual
  (params (bEnable :type Boolean))
  (Utilities|IsValid (Variables|Data|GetOutOfBoundsVisual)
    (:Is%20Valid
      (Default|EnableOutOfBoundsVisual (Variables|Data|GetOutOfBoundsVisual) bEnable))))

(fn GetOutOfBoundsVisual
  (return (Variables|Data|GetOutOfBoundsVisual)))