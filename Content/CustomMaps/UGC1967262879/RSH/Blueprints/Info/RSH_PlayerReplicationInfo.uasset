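; Per-player replication info for the RSH attack/defend MCOM mode, holding role, armory state, XP and rank.
; Role, battlefield, MCOM and bayonet-hit actions run on the server, with clients forwarding through server RPCs.
; The client saves stats and XP, reports total XP to the server, and caches rank from game logic with a rank-up sound.
; Overlapping out-of-bounds volumes are counted, driving a warning and timed suicide.
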(event Custom|ClientAttackersWin
  (WinEvents|AttackersWin))

(event Custom|ServerDisarmMCOM
  (params (MCOMIndex :type Byte))
  (MCOM|DisarmMCOM MCOMIndex))

(event Custom|ServerGoToBattlefield
  (RoleRooms|GotoBattlefield))

(event Custom|ServerSetRoleIndex
  (params (NewRoleIndex :type Byte))
  (Setters|SetRoleIndex NewRoleIndex))

(event Custom|ServerArmMCOM
  (params (MCOMIndex :type Byte))
  (MCOM|ArmMCOM MCOMIndex))

(event Custom|ServerResetRoleIndex
  (Setters|ResetRoleIndex))

(event Custom|ClientAddXP
  (params (AdditionalXP :type Integer))
  (Stats|AddTotalXpStat AdditionalXP)
  (CallFunction|ServerUpdateTotalXP (GettersStats|GetTotalXPStat)))

(event Custom|ClientDefendersWin
  (WinEvents|DefendersWin))

(event Custom|ServerUpdateTotalXP
  (params (NewTotalXP :type Integer))
  (Variables|Stats|SetTotalXp NewTotalXP))

(event Custom|ServerRegisterBayoHit
  (params (HitChar :type Character%20Object%20Reference) (DamagingBayo :type RSH%20Bayo%20Attachment%20Object%20Reference))
  (CustomItems|RegisterBayoHit HitChar DamagingBayo))

(event EventPlayerDied
  (|CallParentFunction)
  (Variables|Data|SetbDiedInArmory (Variables|DataReplicated|GetbIsInArmory))
  (Setters|ResetRoleIndex))

(event EventPlayerSpawned
  (bind (_character _bisvalid) (CallFunction|GetPlayerCharacter))
  (|CallParentFunction)
  (Variables|DataReplicated|SetbIsInArmory true)
  (if _bisvalid
    (Variables|/Script/Engine.Actor|SetbCanBeDamaged _character false)))

(event EventLocalTick
  (params (DeltaTime :type Float%20%28single-precision%29))
  (|CallParentFunction DeltaTime)
  (Bounds|UpdateOutOfBounds)
  (CallFunction|AddPMFConstantLog "TotalXP" (Utilities|String|ToString(Integer) (GettersStats|GetTotalXPStat)))
  (CallFunction|AddPMFConstantLog "RankName" (Default|GetRankNamebyXP (Variables|Data|GetRSHGameLogic) (GettersStats|GetTotalXPStat)))
  (CallFunction|AddPMFConstantLog "CahcedRankName" (Variables|Data|GetCachedRankName)))

(event EventAddScore
  (params (AdditionalScore :type Integer))
  (|CallParentFunction AdditionalScore)
  (CallFunction|ClientAddXP AdditionalScore))

(event EventClientDied
  (|CallParentFunction)
  (Variables|Data|SetIsOutOfBoundsCount 0))

(event EventClientInitialization
  (|CallParentFunction)
  (Rank|RecacheRank))

(event EventBeginPlay
  (Utilities|FlowControl|Sequence
    (:then_0
      (bind _asrsh_game_logic (Utilities|Casting|CastToRSH_GameLogic (CallFunction|GetPMFGameLogic)))
      (Variables|Data|SetRSHGameLogic _asrsh_game_logic))
    (:then_1
      (|CallParentFunction))))

(fn ConstructionScript
  (|CallParentFunction))

(fn ArmMCOM
  (params (MCOMIndex :type Byte))
  (if (Networking|IsServer)
    (Default|ArmMCOM (.MCOMManager (CallFunction|GetMCOMManager)) MCOMIndex self)
    (else
      (CallFunction|ServerArmMCOM MCOMIndex)
      (Stats|IncrPlantedBombStat))))

(fn GetIsinArmory
  (return (Variables|DataReplicated|GetbIsInArmory)))

(fn GetRoleIndex
  (return (Variables|DataReplicated|GetRoleIndex)))

(fn SetRoleIndex
  (params (NewRoleIndex :type Byte))
  (if (Networking|IsServer)
    (Utilities|FlowControl|Sequence
      (:then_0
        (Variables|DataReplicated|SetRoleIndex NewRoleIndex))
      (:then_1
        (Default|SpawnDefaultLoadOut (Variables|Data|GetRSHGameLogic) self (.DefaultRoleLoadout (Default|GetRoleDefaultLoadout (Variables|Data|GetRSHGameLogic) (Variables|DataReplicated|GetRoleIndex) (Info|IsDefender))))
        (Class|PavlovGameLogic|SetPlayerVitality (Variables|Data|GetRSHGameLogic) (CallFunction|GetOwningPlayerState) -1 (select (.RoleHasArmor (Default|GetRoleHasArmor (Variables|Data|GetRSHGameLogic) (Variables|DataReplicated|GetRoleIndex) (Info|IsDefender))) 1 0) (select (.RoleHasHelmet (Default|GetRoleHasHelmet (Variables|Data|GetRSHGameLogic) (Variables|DataReplicated|GetRoleIndex) (Info|IsDefender))) 1 0))))
    (else
      (CallFunction|ServerSetRoleIndex NewRoleIndex))))

(fn ResetRoleIndex
  (if (Networking|IsServer)
    (Variables|DataReplicated|SetRoleIndex 255)
    (else
      (CallFunction|ServerResetRoleIndex))))

(fn IsAttacker
  (bind _asrsh_game_logic (Utilities|Casting|CastToRSH_GameLogic (CallFunction|GetPMFGameLogic))
    (:then
      (return (== (Default|GetAttackersTeamIndex _asrsh_game_logic) (CallFunction|GetTeamIndex))))
    (:CastFailed
      (return true))))

(fn IsDefender
  (return (not (Info|IsAttacker))))

(fn GetRSHRole
  (bind _roleindex (Info|GetRoleIndex))
  (bind _returnvalue (Math|Conversions|ToInteger(Byte) _roleindex))
  (bind _asrsh_game_logic (Utilities|Casting|CastToRSH_GameLogic (CallFunction|GetPMFGameLogic))
    (:then
      (if (!= (Info|GetRoleIndex) 255)
        (if (Utilities|Array|IsValidIndex (select (Info|IsDefender) (Default|GetDefendersTeamRoles _asrsh_game_logic) (Default|GetAttackersTeamRoles _asrsh_game_logic)) _returnvalue)
          (return (Utilities|Array|Get(acopy) (select (Info|IsDefender) (Default|GetDefendersTeamRoles _asrsh_game_logic) (Default|GetAttackersTeamRoles _asrsh_game_logic)) _returnvalue) true)
          (else
            (return "" false)))
        (else
          (return "" false))))
    (:CastFailed
      (return "" false))))

(fn GotoBattlefield
  (bind (_character _bisvalid) (CallFunction|GetPlayerCharacter))
  (if (Networking|IsServer)
    (Variables|DataReplicated|SetbIsInArmory false)
    (if _bisvalid
      (Variables|/Script/Engine.Actor|SetbCanBeDamaged _character true))
    (else
      (CallFunction|ServerGotoBattlefield))))

(fn DisarmMCOM
  (params (MCOMIndex :type Byte))
  (if (Networking|IsServer)
    (Default|DisarmedMCOM (.MCOMManager (CallFunction|GetMCOMManager)) MCOMIndex self)
    (else
      (CallFunction|ServerDisarmMCOM MCOMIndex)
      (Stats|IncrDefusedBombStat))))

(fn DefendersWin
  (if (Networking|IsServer)
    (CallFunction|ClientDefendersWin)))

(fn AttackersWin
  (if (Networking|IsServer)
    (CallFunction|ClientAttackersWin)))

(fn SpawnRoundOverScreen
  (bind _self self)
  (Game|SpawnActorfromClass (Variables|Config|GetRSHRoundOverScreen) (Math|Transform|MakeTransform "0, 0, 0") "AlwaysSpawn" _self _self 0))

(fn GetRSHSaveData
  (bind _asrsh_save_game (Utilities|Casting|CastToRSH_SaveGame (Variables|Default|GetPMFSaveData))
    (:then
      (return _asrsh_save_game true))
    (:CastFailed
      (return 0 false))))

(fn IncrPlantedBombStat
  (bind (_asrsh_save_game _bvalid) (INfo|GetRSHSaveData))
  (if _bvalid
    (Math|Integer|IncrementInt (Variables|/Game/CustomMaps/UGC1967262879/RSH/Blueprints/Saving/RSH_SaveGame.RSH_SaveGame_C|GetNumOfTimesPlantedBomb _asrsh_save_game)
      (:%20%20
        (CallFunction|SaveGameInfo)))))

(fn IncrDefusedBombStat
  (bind (_asrsh_save_game _bvalid) (INfo|GetRSHSaveData))
  (if _bvalid
    (Math|Integer|IncrementInt (Variables|/Game/CustomMaps/UGC1967262879/RSH/Blueprints/Saving/RSH_SaveGame.RSH_SaveGame_C|GetNumOfTimesPlantedBomb _asrsh_save_game)
      (:%20%20
        (CallFunction|SaveGameInfo)))))

(fn AddTotalXpStat
  (params (AdditionalXP :type Integer))
  (bind (_asrsh_save_game _bvalid) (INfo|GetRSHSaveData))
  (if _bvalid
    (LocalVariables|SetOldCachedRankName (Variables|Data|GetCachedRankName))
    (Variables|/Game/CustomMaps/UGC1967262879/RSH/Blueprints/Saving/RSH_SaveGame.RSH_SaveGame_C|SetTotalXp _asrsh_save_game (Math|Integer|Max(Integer) (+ AdditionalXP (Variables|/Game/CustomMaps/UGC1967262879/RSH/Blueprints/Saving/RSH_SaveGame.RSH_SaveGame_C|GetTotalXp _asrsh_save_game))))
    (CallFunction|SaveGameInfo)
    (Rank|RecacheRank)
    (if (> (Utilities|String|Len (LocalVariables|GetOldCachedRankName)) 0) ; If we had a rank cached
      (if (Utilities|Enum|NotEqual(Enum) (Variables|Data|GetCachedRankName) (LocalVariables|GetOldCachedRankName)) ; Are we a new rank?
        (Rank|RankedUp)))))

(fn GetPlantedBombStat
  (bind (_asrsh_save_game _bvalid) (INfo|GetRSHSaveData))
  (if _bvalid
    (return (Variables|/Game/CustomMaps/UGC1967262879/RSH/Blueprints/Saving/RSH_SaveGame.RSH_SaveGame_C|GetNumOfTimesPlantedBomb _asrsh_save_game))
    (else
      (return 0))))

(fn GetDefusedBombStat
  (bind (_asrsh_save_game _bvalid) (INfo|GetRSHSaveData))
  (if _bvalid
    (return (Variables|/Game/CustomMaps/UGC1967262879/RSH/Blueprints/Saving/RSH_SaveGame.RSH_SaveGame_C|GetNumOfTimesDefusedBomb _asrsh_save_game))
    (else
      (return 0))))

(fn GetTotalXPStat
  (bind (_asrsh_save_game _bvalid) (INfo|GetRSHSaveData))
  (if (CallFunction|IsLocalPRI)
    (if _bvalid
      (return (Variables|/Game/CustomMaps/UGC1967262879/RSH/Blueprints/Saving/RSH_SaveGame.RSH_SaveGame_C|GetTotalXp _asrsh_save_game))
      (else
        (return (Variables|Stats|GetTotalXp))))
    (else
      (return (Variables|Stats|GetTotalXp)))))

(fn RegisterBayoHit
  (params (HitChar :type Character%20Object%20Reference) (DamagingBayo :type RSH%20Bayo%20Attachment%20Object%20Reference))
  (Utilities|IsValid HitChar
    (:Is%20Valid
      (Utilities|IsValid DamagingBayo
        (:Is%20Valid
          (if (Networking|IsServer)
            (Default|ServerGetBayoHit DamagingBayo HitChar self)
            (else
              (CallFunction|ServerRegisterBayoHit HitChar DamagingBayo))))))))

(fn PlayerHasGoneOutOfBounds
  (params (BoundsVolume :type RSH%20Volume%20Return%20to%20Battlefield%20Object%20Reference))
  (Variables|Data|SetIsOutOfBoundsCount (+ (Variables|Data|GetIsOutOfBoundsCount) 1))
  (if (== (Variables|Data|GetIsOutOfBoundsCount) 1) ; If this is the first one, set the timer!
    (Variables|Data|SetOutOfBoundsStartTime (GameState|GetServerWorldTimeSeconds (Game|GetGameState)))
    (bind _asrsh_character_proxy_info (Utilities|Casting|CastToRSH_CharacterProxyInfo (.SpawnedCharacterProxyInfo (CallFunction|GetCharacterProxyInfo))))
    (Default|EnableOutOfBoundsVisual _asrsh_character_proxy_info true)
    (bind _asrsh_sound_manager (Utilities|Casting|CastToRSH_SoundManager (.PMFSoundManager (CallFunction|GetPMFSoundManager))))
    (Default|PlayReturntoBattlefieldSound _asrsh_sound_manager)))

(fn UpdateOutOfBounds
  (if (> (Variables|Data|GetIsOutOfBoundsCount) 0)
    (if (>= (- (GameState|GetServerWorldTimeSeconds (Game|GetGameState)) (Variables|Data|GetOutOfBoundsStartTime)) (Variables|Config|GetOutOfBoundsTime))
      (CallFunction|Suicide)
      (Variables|Data|SetIsOutOfBoundsCount 0) ; Stops Server RPC spam
    )))

(fn PlayerHasReturnedfromOutOfBounds
  (params (BoundsVolume :type RSH%20Volume%20Return%20to%20Battlefield%20Object%20Reference))
  (if (> (Variables|Data|GetIsOutOfBoundsCount) 0)
    (Variables|Data|SetIsOutOfBoundsCount (- (Variables|Data|GetIsOutOfBoundsCount) 1))
    (if (== (Variables|Data|GetIsOutOfBoundsCount) 0)
      (bind _asrsh_character_proxy_info (Utilities|Casting|CastToRSH_CharacterProxyInfo (.SpawnedCharacterProxyInfo (CallFunction|GetCharacterProxyInfo))))
      (Default|EnableOutOfBoundsVisual _asrsh_character_proxy_info false))))

(fn GetRankTexture
  (return (Variables|Data|GetCachedRankTexture)))

(fn OnRepTotalXp
  (Rank|RecacheRank))

(fn GetRankName
  (return (Variables|Data|GetCachedRankName)))

(fn GetNextRankXP
  (return (Variables|Data|GetCachedNextRankXP)))

(fn RecacheRank
  (Utilities|IsValid (Variables|Data|GetRSHGameLogic)
    (:Is%20Valid
      (Utilities|FlowControl|Sequence
        (:then_0
          (Variables|Data|SetCachedRankName (Default|GetRankNamebyXP (Variables|Data|GetRSHGameLogic) (GettersStats|GetTotalXPStat))))
        (:then_1
          (Variables|Data|SetCachedRankTexture (Default|GetRankIconbyXP (Variables|Data|GetRSHGameLogic) (GettersStats|GetTotalXPStat))))
        (:then_2
          (Variables|Data|SetCachedNextRankXP (Default|GetNextRankXPbyXP (Variables|Data|GetRSHGameLogic) (GettersStats|GetTotalXPStat))))))))

(fn RankedUp
  (bind _asrsh_sound_manager (Utilities|Casting|CastToRSH_SoundManager (.PMFSoundManager (CallFunction|GetPMFSoundManager))))
  (Default|PlayRankUpSound _asrsh_sound_manager))