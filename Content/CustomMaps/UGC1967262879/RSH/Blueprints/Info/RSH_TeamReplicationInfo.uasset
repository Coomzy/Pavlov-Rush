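; RSH team replication info Blueprint that adds an optional pool of respawn tickets to a team.
; When tickets are enabled, functions set, add and consume them; when disabled, those changes are ignored and ticket checks always pass.
; CanPlayerRespawn is overridden to refuse respawns once tickets run out, otherwise deferring to the parent class's rule.
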(fn ConstructionScript
  (|CallParentFunction))

(fn GetUseRespawnTickets
  (return (Variables|DataReplicated|GetbUseRespawnTickets)))

(fn GetRespawnTickets
  (return (Variables|DataReplicated|GetRespawnTickets)))

(fn ConsumeRespawnTicket
  (if (Variables|DataReplicated|GetbUseRespawnTickets)
    (Math|Integer|DecrementInt (Variables|DataReplicated|GetRespawnTickets))))

(fn SetRespawnTickets
  (params (NewRespawnTickets :type Integer))
  (if (Variables|DataReplicated|GetbUseRespawnTickets)
    (Variables|DataReplicated|SetRespawnTickets NewRespawnTickets)))

(fn AddRespawnTickets
  (params (AdditionalRespawnTickets :type Integer))
  (if (Variables|DataReplicated|GetbUseRespawnTickets)
    (Variables|DataReplicated|SetRespawnTickets (+ AdditionalRespawnTickets (Variables|DataReplicated|GetRespawnTickets)))))

(fn CanRespawnUsingTickets
  (if (Variables|DataReplicated|GetbUseRespawnTickets)
    (return (> (Variables|DataReplicated|GetRespawnTickets) 0))
    (else
      (return true))))

(fn SetUseRespawnTickets
  (params (NewUseRespawnTickets :type Boolean))
  (Variables|DataReplicated|SetbUseRespawnTickets NewUseRespawnTickets))

(fn CanPlayerRespawn
  (params (PRI :type PMF%20Player%20Replication%20Info%20Object%20Reference))
  (if (Info|HasRespawnTicketsLeft)
    (bind _bcanrespawn (|CallParentFunction PRI))
    (return _bcanrespawn)
    (else
      (return false))))

(fn HasRespawnTicketsLeft
  (if (Variables|DataReplicated|GetbUseRespawnTickets)
    (return (> (Variables|DataReplicated|GetRespawnTickets) 0))
    (else
      (return true))))